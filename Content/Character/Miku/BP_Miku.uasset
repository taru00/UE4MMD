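; Miku character Blueprint that sets up a cloned mesh and can spin back and forth.
; On BeginPlay it hands its Mesh to the ClonedCharacter component as the parent mesh and has it generate the clone.
; While RotationCycle is set, Tick drives a single axis of the RotatingMovement rotation rate with a game-time sine wave, so the spin periodically reverses direction.
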(event EventBeginPlay
  (bind _clonedcharacter (Variables|Default|GetClonedCharacter))
  (Variables|Default|SetParentsMeshComponent _clonedcharacter (Variables|Character|GetMesh))
  (CallFunction|GenerateClonedMesh _clonedcharacter))

(event Collision|EventActorBeginOverlap
  (params (OtherActor :type Actor%20Object%20Reference)))

(event EventTick
  (params (DeltaSeconds :type Float%20%28single-precision%29))
  (if (Variables|Default|GetRotationCycle)
    (Variables|/Script/Engine.RotatingMovementComponent|SetRotationRate (Variables|Default|GetRotatingMovement) (Math|Rotator|MakeRotator 0.0 0.0 (* (Math|Trig|Sin(Radians) (* (Utilities|Time|GetGameTimeinSeconds) 5.0)) 1.8e+02)))))

(fn ConstructionScript)